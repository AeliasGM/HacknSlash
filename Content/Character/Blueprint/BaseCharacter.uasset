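; Base character for one-handed weapon and shield melee combat, with attack, block, jump and walk/run toggle inputs.
; Attacks open a timed weapon-collision window with a montage, then spend stamina; the attack type is currently fixed to horizontal.
; Blocking slows movement and enables shield collision.
; Hit and blocked events play montage sections, with the character's own blocked swing disabling weapon collision and playing in reverse.
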(event `self.ReceiveBeginPlay`
  (`self.Block`)
  (bind _as1h_weapon (cast `/Game/Character/Weaponry/1H_Weapon` (`ChildActorComponent.ChildActor` (`self.Weapon`))))
  (set `self.MyWeapon` _as1h_weapon)
  (bind _asshield (cast `/Game/Character/Weaponry/Shield` (`ChildActorComponent.ChildActor` (`self.Shield`))))
  (set `self.MyShield` _asshield)
  (`KismetSystemLibrary.PrintString` (`KismetStringLibrary.Conv_IntToString` (- (enumcount `EVitalNames`) (`KismetArrayLibrary.Array_Length` (`self.Vitals`))))))

(event `self.ReceiveTick`
  (params (DeltaSeconds :type "Float (single-precision)"))
  (set `self.isInAir` (`NavMovementComponent.IsFalling` (`self.CharacterMovement`)))
  (if (not (`self.isInAir`))
    (set `self.isJumping` false)))

(event `InputAction|Attack_back`
  (params (Key :type "Key Structure"))
  (:`Pressed`
    (`self.Attack`)))

(event `InputAction|Block`
  (params (Key :type "Key Structure"))
  (:`Pressed`
    ;[1 1 1] set stamina recovery rate
    (`self.Block`))
  (:`Released`
    (`self.BlockEnd`)))

(event `Attack`
  ;[1 1 1] Attack
  (if (not (`self.IsAttacking`))
    (set `self.IsAttacking` true)
    (`/Game/Character/Weaponry/1H_Weapon.EnableCollision` (`self.MyWeapon`) true)
    (bind _output_get (set `self.AttackType` "NewEnumerator1"))
    (switch `/Game/Character/Weaponry/AttackTypes` _output_get
      (:`NewEnumerator0`
        (set `self.AnimSection` "Downward"))
      (:`NewEnumerator1`
        (set `self.AnimSection` "Horizontal"))
      (:`NewEnumerator2`
        (set `self.AnimSection` "Backhand")))
    (`self.PlayAnimMontage` "/Game/Character/Animations/1H_Attack.1H_Attack" 1.0 (`self.AnimSection`))
    (`KismetSystemLibrary.Delay` 1.0)
    (`/Game/Character/Weaponry/1H_Weapon.EnableCollision` (`self.MyWeapon`) false)
    (set `self.IsAttacking` false)
    (`self.StatModifyCurrent` "VN_Stamina" -10.0)
    (bind _returnvalue (`self.GetCurrentPercent` "VN_Stamina"))
    (`KismetSystemLibrary.PrintString` (`KismetStringLibrary.Conv_DoubleToString` _returnvalue))))

(event `Block`
  (set `CharacterMovementComponent.MaxWalkSpeed` 200.0 (`self.CharacterMovement`))
  (`self.PlayAnimMontage` "/Game/Character/Animations/1H_Block.1H_Block" 1.0 "BlockStart")
  (message `/Game/Character/Weaponry/Weaponry.CollisionEnabler` (`self.Shield`) true))

(event `BlockEnd`
  (`self.PlayAnimMontage` "/Game/Character/Animations/1H_Block.1H_Block" 1.0 "BlockEnd")
  (message `/Game/Character/Weaponry/Weaponry.CollisionEnabler` (`self.Shield`) false))

(event `InputAction|Jump`
  (params (Key :type "Key Structure"))
  (:`Pressed`
    (set `self.isJumping` true)
    (`self.Jump`)))

(event `InputAction|Speed`
  (params (Key :type "Key Structure"))
  (bind _charactermovement (`self.CharacterMovement`))
  (:`Pressed`
    (`/Engine/EditorBlueprintResources/StandardMacros.FlipFlop`
      (:`A`
        (set `CharacterMovementComponent.MaxWalkSpeed` 600.0 _charactermovement))
      (:`B`
        (set `CharacterMovementComponent.MaxWalkSpeed` 200.0 _charactermovement)))))

(event `/Game/Character/Weaponry/Weaponry.AttackIn`
  (params (EnemyAttackType :type "/Game/Character/Weaponry/AttackTypes Enum" :default "NewEnumerator0"))
  (`KismetSystemLibrary.PrintString` "HIT")
  ;[1 1 1] IsDead?
  (if (not (`self.IsDead`))
    (switch `/Game/Character/Weaponry/AttackTypes` EnemyAttackType
      (:`NewEnumerator0`
        (set `self.AnimSection` "Impact_Side" :!label _label))
      (:`NewEnumerator1`
        (goto _label))
      (:`NewEnumerator2`
        (set `self.AnimSection` "Impact_Up")))
    (`self.PlayAnimMontage` "/Game/Character/Animations/Weapon_Impact.Weapon_Impact" 1.0 (`self.AnimSection`))
    (message `/Game/Character/Weaponry/Weaponry.CollisionEnabler` (`self.Shield`) false)))

(event `/Game/Character/Weaponry/Weaponry.AttackBlocked`
  (`KismetSystemLibrary.PrintString` "Blocked")
  (`self.PlayAnimMontage` "/Game/Character/Animations/1H_Block.1H_Block" 1.0 "AttackBlocked")
  (`self.Block`))

(event `myAttackBlocked`
  (message `/Game/Character/Weaponry/Weaponry.CollisionEnabler` (`self.Weapon`) false)
  (switch `/Game/Character/Weaponry/AttackTypes` (`self.AttackType`)
    (:`NewEnumerator0`
      (set `self.AnimSection` "Downward_Blocked"))
    (:`NewEnumerator1`
      (set `self.AnimSection` "Horizontal_Blocked"))
    (:`NewEnumerator2`
      (set `self.AnimSection` "Backhand_Blocked")))
  (`self.PlayAnimMontage` "/Game/Character/Animations/1H_Attack.1H_Attack" -1.0 (`self.AnimSection`)))

(fn `UserConstructionScript`)